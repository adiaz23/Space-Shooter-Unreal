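; Player-controlled spaceship pawn for a space shooter, handling movement, twin-gun firing and lives.
; On BeginPlay it adds its Enhanced Input mapping context, and the movement action drives movement input along the ship's right and forward vectors.
; Firing spawns ammo at two spawn points, then blocks further shots until a delay timer re-enables them.
; Each DamageActor event removes a life, and the game mode's PlayerDead is called when lives reach zero.
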(event Custom|DamageActor
  (CallFunction|ReduceLives))

(event Input|EnhancedActionEvents|EnhancedInputActionBP_InputFire
  (params (ActionValue :type Boolean) (ElapsedSeconds :type Float%20%28double-precision%29) (TriggeredSeconds :type Float%20%28double-precision%29) (InputAction :type Input%20Action%20Object%20Reference :default "/Game/Input/BP_InputFire.BP_InputFire"))
  ;[1 1 1] Set Key for player fire
  (if (Variables|Default|GetCanFire)
    (CallFunction|Fire)
    (Utilities|Time|SetTimerbyFunctionName 0 "CanFireTrue" (Variables|Default|GetFireDelay))))

(event Input|EnhancedActionEvents|EnhancedInputActionBP_Movement
  (params (ActionValue :type Vector%202D%20Structure) (ElapsedSeconds :type Float%20%28double-precision%29) (TriggeredSeconds :type Float%20%28double-precision%29) (InputAction :type Input%20Action%20Object%20Reference :default "/Game/Input/BP_Movement.BP_Movement"))
  ;[1 1 1] Set keys for Player movement
  (CallFunction|Move (.x ActionValue) (.y ActionValue)))

(event EventBeginPlay
  ;[1 1 1] Get Player Inputs
  (CallFunction|GetPlayerInputs))

(fn ConstructionScript)

(fn Fire
  (Game|SpawnActorfromClass (Variables|Default|GetAmmo) (Transformation|GetWorldTransform (Variables|Default|GetSpawn_Ammo1)) "Undefined" "MultiplyWithRoot" 0 0)
  (Game|SpawnActorfromClass (Variables|Default|GetAmmo) (Transformation|GetWorldTransform (Variables|Default|GetSpawn_Ammo2)) "Undefined" "MultiplyWithRoot" 0 0)
  (Variables|Default|SetCanFire false))

(fn Move
  (params (horizontalMove :type Float%20%28double-precision%29) (verticalMove :type Float%20%28double-precision%29))
  (Pawn|Input|AddMovementInput (Transformation|GetActorRightVector) horizontalMove false)
  (Pawn|Input|AddMovementInput (Transformation|GetActorForwardVector) verticalMove false))

(fn GetPlayerInputs
  (bind _asplayer_controller (Utilities|Casting|CastToPlayerController (Pawn|GetController)))
  (Utilities|IsValid (PlayerController|LocalPlayerSubsystems|GetEnhancedInputLocalPlayerSubsystem _asplayer_controller)
    (:Is%20Valid
      (Input|AddMappingContext (PlayerController|LocalPlayerSubsystems|GetEnhancedInputLocalPlayerSubsystem _asplayer_controller) "/Game/Input/BP_Input_Mapping.BP_Input_Mapping" 0 "(bIgnoreAllPressedKeysUntilRelease=True,bForceImmediately=False,bNotifyUserSettings=False)"))))

(fn CanFireTrue
  (Variables|Default|SetCanFire true))

(fn ReduceLives
  (bind _output_get (Variables|Default|SetLives (- (Variables|Default|GetLives) 1)))
  (if (== _output_get 0)
    (bind _asbp_game_mode_space_shooter (Utilities|Casting|CastToBP_GameMode_SpaceShooter (Game|GetGameMode)))
    (Default|PlayerDead _asbp_game_mode_space_shooter)))