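; BP_Ship_Ammo is a ship projectile that flies straight ahead and explodes on contact with a Pawn.
; Tick calls Movement, which offsets the location along the forward vector by Speed and delta time, without sweeping.
; Overlapping a Pawn spawns an explosion emitter and 2D sound, then destroys the projectile after a short delay.
; The file applies no damage to the overlapped Pawn.
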(event Collision|EventActorBeginOverlap
  (params (OtherActor :type Actor%20Object%20Reference))
  (Utilities|Casting|CastToPawn OtherActor)
  (Effects|SpawnEmitteratLocation "/Game/StarterContent/Particles/P_Explosion.P_Explosion" (Transformation|GetActorLocation))
  (Audio|PlaySound2D "/Game/StarterContent/Audio/Explosion01.Explosion01" 1.0 1.0 0.0 0 0)
  (Utilities|FlowControl|Delay 0.2)
  (Actor|DestroyActor))

(event EventTick
  (params (DeltaSeconds :type Float%20%28single-precision%29))
  ;[1 1 1] Ammo Movement
  (CallFunction|Movement DeltaSeconds))

(fn ConstructionScript)

(fn Movement
  (params (deltaSeconds :type Float%20%28double-precision%29))
  (Transformation|SetActorLocation (+ (Transformation|GetActorLocation) (* (Transformation|GetActorForwardVector) (* deltaSeconds (Variables|Default|GetSpeed)))) false false))