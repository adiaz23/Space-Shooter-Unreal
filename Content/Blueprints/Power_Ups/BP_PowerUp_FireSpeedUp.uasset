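; Fire rate power-up that speeds up the player ship's shooting.
; On BeginPlay it casts the player character to BP_Space_Ship and caches it.
; ApplyPowerUp lowers the ship's FireDelay by a fixed step, but only while the delay is at or above a minimum threshold.
; Its own overlap and tick events are disabled, and the file does not show what triggers ApplyPowerUp.
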(event EventBeginPlay
  (bind _asbp_space_ship (Utilities|Casting|CastToBP_Space_Ship (Game|GetPlayerCharacter 0)))
  (Variables|Default|SetPlayer _asbp_space_ship))

(event Collision|EventActorBeginOverlap
  (params (OtherActor :type Actor%20Object%20Reference))
  (|CallParentFunction OtherActor) ; This node is disabled and will not be called.\nDrag off pins to build functionality.
)

(event EventTick
  (params (DeltaSeconds :type Float%20%28single-precision%29))
  (|CallParentFunction DeltaSeconds) ; This node is disabled and will not be called.\nDrag off pins to build functionality.
)

(event EventApplyPowerUp
  (params (Other%20Actor :type Actor%20Object%20Reference))
  (bind _player (Variables|Default|GetPlayer))
  ;[1 1 1] Set PowerUp to reduce the FireDelay
  (if (>= (Variables|/Game/Blueprints/Characters/Player/BP_Space_Ship.BP_Space_Ship_C|GetFireDelay _player) 0.2)
    (Variables|/Game/Blueprints/Characters/Player/BP_Space_Ship.BP_Space_Ship_C|SetFireDelay _player (- (Variables|/Game/Blueprints/Characters/Player/BP_Space_Ship.BP_Space_Ship_C|GetFireDelay _player) 0.04))))

(fn ConstructionScript
  (|CallParentFunction))