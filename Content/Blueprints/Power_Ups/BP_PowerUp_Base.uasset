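; Base power-up actor that moves through the level and boosts the player's walk speed on pickup.
; Tick moves it along MovementVector at Speed, without sweeping.
; Overlap with a "Player"-tagged actor calls ApplyPowerUp, plays a 2D sound and destroys the power-up after a short delay.
; ApplyPowerUp adds WalkSpeed to player 0's MaxWalkSpeed with no revert, ignoring the overlapping actor passed in.
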(event Custom|ApplyPowerUp
  (params (Other%20Actor :type Actor%20Object%20Reference))
  (bind _returnvalue (Game|GetPlayerCharacter 0))
  (bind _charactermovement (Variables|/Script/Engine.Character|GetCharacterMovement _returnvalue))
  ;[1 1 1] Apply Power Up
  (Variables|/Script/Engine.CharacterMovementComponent|SetMaxWalkSpeed _charactermovement (+ (Variables|Default|GetWalk%20Speed) (Variables|/Script/Engine.CharacterMovementComponent|GetMaxWalkSpeed _charactermovement))))

(event EventTick
  (params (DeltaSeconds :type Float%20%28single-precision%29))
  ;[1 1 1] Power Up movement
  (CallFunction|Move DeltaSeconds))

(event Collision|EventActorBeginOverlap
  (params (OtherActor :type Actor%20Object%20Reference))
  ;[1 1 1] Call Apply Power Up and Destroy it
  (if (Actor|ActorHasTag OtherActor "Player")
    (CallFunction|ApplyPowerUp OtherActor)
    (Audio|PlaySound2D "/Game/Assests/Sounds/Effects/arcade-game-power-up-epic-stock-media-1-00-00.arcade-game-power-up-epic-stock-media-1-00-00" 1.0 1.0 0.0 0 0)
    (Utilities|FlowControl|Delay 0.1)
    (Actor|DestroyActor)))

(fn ConstructionScript)

(fn Move
  (params (Delta%20Time :type Float%20%28double-precision%29))
  (Transformation|SetActorLocation (+ (Transformation|GetActorLocation) (* (* Delta%20Time (Variables|Default|GetSpeed)) (Variables|Default|GetMovementVector))) false false))