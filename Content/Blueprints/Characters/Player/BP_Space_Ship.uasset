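; Player-controlled spaceship pawn for a space shooter, with movement, firing and lives.
; Enhanced Input drives movement along the actor's right and forward vectors and fires a spawned projectile with laser sound, using a timer-based cooldown.
; Overlapping an "Enemy"-tagged actor calls the ReduceLives dispatcher, whose bound event decrements lives.
; At zero lives, the ship briefly waits, destroys itself and notifies BP_GameMode_SpaceShooter.
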(event Custom|ReducesLives
  ;[1 1 1] Get Player Inputs and set up Reduce Lives Dispatcher
  (bind _output_get (Variables|Default|SetLives (- (Variables|Default|GetLives) 1)))
  (if (== _output_get 0)
    (Utilities|FlowControl|Delay 0.1)
    (Actor|DestroyActor)
    (bind _asbp_game_mode_space_shooter (Utilities|Casting|CastToBP_GameMode_SpaceShooter (Game|GetGameMode)))
    (Default|PlayerDead _asbp_game_mode_space_shooter)))

(event Input|EnhancedActionEvents|EnhancedInputActionBP_InputFire
  (params (ActionValue :type Boolean) (ElapsedSeconds :type Float%20%28double-precision%29) (TriggeredSeconds :type Float%20%28double-precision%29) (InputAction :type Input%20Action%20Object%20Reference :default "/Game/Blueprints/Input/BP_InputFire.BP_InputFire"))
  ;[1 1 1] Set Key for player fire
  (if (Variables|Default|GetCanFire)
    (CallFunction|Fire)
    (Utilities|Time|SetTimerbyFunctionName 0 "CanFireTrue" (Variables|Default|GetFireDelay))))

(event Input|EnhancedActionEvents|EnhancedInputActionBP_Movement
  (params (ActionValue :type Vector%202D%20Structure) (ElapsedSeconds :type Float%20%28double-precision%29) (TriggeredSeconds :type Float%20%28double-precision%29) (InputAction :type Input%20Action%20Object%20Reference :default "/Game/Blueprints/Input/BP_Movement.BP_Movement"))
  ;[1 1 1] Set keys for Player movement
  (CallFunction|Move (.x ActionValue) (.y ActionValue)))

(event Collision|EventActorBeginOverlap
  (params (OtherActor :type Actor%20Object%20Reference))
  ;[1 1 1] Reduce lives
  (if (Actor|ActorHasTag OtherActor "Enemy")
    (Default|CallReduceLives)))

(event EventBeginPlay
  ;[1 1 1] Get Player Inputs and set up Reduce Lives Dispatcher
  (CallFunction|GetPlayerInputs)
  (EventDispatchers|BindEventtoReduceLives (delegate Custom|ReducesLives)))

(fn ConstructionScript)

(fn Fire
  (Game|SpawnActorfromClass (Variables|Default|GetAmmo) (Transformation|GetWorldTransform (Variables|Default|GetSpawn_Ammo1)) "Undefined" "MultiplyWithRoot" 0 0)
  (Audio|PlaySound2D "/Game/Assests/Sounds/Effects/Laser-gun-shot.Laser-gun-shot" 0.2 1.0 0.0 0 0 false)
  (Variables|Default|SetCanFire false))

(fn Move
  (params (horizontalMove :type Float%20%28double-precision%29) (verticalMove :type Float%20%28double-precision%29))
  (Pawn|Input|AddMovementInput (Transformation|GetActorRightVector) horizontalMove false)
  (Pawn|Input|AddMovementInput (Transformation|GetActorForwardVector) verticalMove false))

(fn GetPlayerInputs
  (bind _asplayer_controller (Utilities|Casting|CastToPlayerController (Pawn|GetController)))
  (Utilities|IsValid (PlayerController|LocalPlayerSubsystems|GetEnhancedInputLocalPlayerSubsystem _asplayer_controller)
    (:Is%20Valid
      (Input|AddMappingContext (PlayerController|LocalPlayerSubsystems|GetEnhancedInputLocalPlayerSubsystem _asplayer_controller) "/Game/Blueprints/Input/BP_Input_Mapping.BP_Input_Mapping" 0 "(bIgnoreAllPressedKeysUntilRelease=True,bForceImmediately=False,bNotifyUserSettings=False)"))))

(fn CanFireTrue
  (Variables|Default|SetCanFire true))