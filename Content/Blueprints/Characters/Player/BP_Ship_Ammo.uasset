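; BP_Ship_Ammo is a projectile actor for the player's ship that flies straight ahead and removes itself on hitting a tagged actor.
; Tick calls Movement, which offsets the location along the forward vector by Speed and delta time, without sweeping.
; Beginning an overlap with an actor carrying the configured Tag triggers a very brief delay, then Destroy removes the projectile.
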(event Collision|EventActorBeginOverlap
  (params (OtherActor :type Actor%20Object%20Reference))
  ;[1 1 1] Destroy Ammo
  (if (Actor|ActorHasTag OtherActor (Variables|Default|GetTag))
    (Utilities|FlowControl|Delay 0.01)
    (CallFunction|Destroy)))

(event EventTick
  (params (DeltaSeconds :type Float%20%28single-precision%29))
  ;[1 1 1] Ammo Movement
  (CallFunction|Movement DeltaSeconds))

(fn ConstructionScript)

(fn Movement
  (params (deltaSeconds :type Float%20%28double-precision%29))
  (Transformation|SetActorLocation (+ (Transformation|GetActorLocation) (* (Transformation|GetActorForwardVector) (* deltaSeconds (Variables|Default|GetSpeed)))) false false))

(fn Destroy
  (Actor|DestroyActor))