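; Base enemy actor for a space shooter that flies straight along its initial forward vector and fires at a regular interval.
; Tick moves it without sweep and runs a timer that spawns the Ammo class at SpawnPoint1, matching the enemy's rotation.
; Overlapping a Player-tagged actor calls the OnEnemyDestroy dispatcher, whose bound handler destroys the actor after a short delay, and notifies BP_GameMode_SpaceShooter.
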(event Custom|Destroyed_Event
  ;[1 1 1] Destroy Enemy
  (Utilities|FlowControl|Delay 0.1)
  (Actor|DestroyActor))

(event EventBeginPlay
  ;[1 1 1] Destroy Enemy
  (Variables|Default|SetMovementVector (Transformation|GetActorForwardVector))
  (EventDispatchers|BindEventtoOnEnemyDestroy (delegate Custom|Destroyed_Event)))

(event EventTick
  (params (DeltaSeconds :type Float%20%28single-precision%29))
  ;[1 1 1] Movement and Fire functions
  (CallFunction|Movement DeltaSeconds)
  (bind _output_get (Variables|Default|SetShootCurrentTime (+ DeltaSeconds (Variables|Default|GetShootCurrentTime))))
  (if (> _output_get (Variables|Default|GetDelayShoot))
    (Variables|Default|SetShootCurrentTime 0.0)
    (CallFunction|Fire)))

(event Collision|EventActorBeginOverlap
  (params (OtherActor :type Actor%20Object%20Reference))
  ;[1 1 1] On collision
  (if (Utilities|Array|ContainsItem (Variables|/Script/Engine.Actor|GetTags OtherActor) "Player")
    (Default|CallOnEnemyDestroy)
    (bind _asbp_game_mode_space_shooter (Utilities|Casting|CastToBP_GameMode_SpaceShooter (Game|GetGameMode)))
    (Default|EnemyDestroyed _asbp_game_mode_space_shooter)))

(fn ConstructionScript)

(fn Movement
  (params (Delta%20Time :type Float%20%28double-precision%29))
  (Transformation|SetActorLocation (+ (Transformation|GetActorLocation) (* (* Delta%20Time (Variables|Default|GetSpeed)) (Variables|Default|GetMovementVector))) false false))

(fn Fire
  (bind _returnvalue (Game|SpawnActorfromClass (Variables|Default|GetAmmo) (Transformation|GetWorldTransform (Variables|Default|GetSpawnPoint1)) "Undefined" "MultiplyWithRoot" 0 0))
  (Transformation|SetActorRotation _returnvalue (Transformation|GetActorRotation)))