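; Enemy spawner for the space shooter that periodically spawns a random enemy on a looping timer.
; The enemy class is picked by a random integer bounded by the game mode's Level and clamped to the available types (Base, H, S).
; Enemies appear at random SpawnPoint-tagged components on the spawner.
; Spawning of any type pauses while more than two BP_Enemy_H actors exist.
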(event Custom|Spawn
  ;[1 1 1] Spawn Enemy
  (CallFunction|SpawnEnemy))

(event EventBeginPlay
  ;[1 1 1] Spawn Enemy
  (Utilities|Time|SetTimerbyEvent (delegate Custom|Spawn) (Variables|Default|GetSpawnTime) true)
  ;[1 1 1] Save Game Mode in Variable
  (bind _asbp_game_mode_space_shooter (Utilities|Casting|CastToBP_GameMode_SpaceShooter (Game|GetGameMode)))
  (Variables|Default|SetGame%20Mode _asbp_game_mode_space_shooter))

(fn ConstructionScript)

(fn SpawnEnemy
  (bind _returnvalue (Actor|GetComponentsbyTag "/Script/Engine.SceneComponent" "SpawnPoint"))
  (bind _class (CallFunction|GetClasstoSpawn (Math|Random|RandomInteger (Variables|/Game/Blueprints/BP_GameMode_SpaceShooter.BP_GameMode_SpaceShooter_C|GetLevel (Variables|Default|GetGame%20Mode)))))
  (bind _outactors (Actor|GetAllActorsOfClass "/Game/Blueprints/Characters/Enemies/BP_Enemy_H.BP_Enemy_H_C"))
  (if (<= (Utilities|Array|Length _outactors) 2)
    (bind _returnvalue_2 (Game|SpawnActorfromClass _class (Transformation|GetWorldTransform (Utilities|Array|Get(acopy) _returnvalue (Math|Random|RandomInteger (Utilities|Array|Length _returnvalue)))) "AdjustIfPossibleButAlwaysSpawn" "MultiplyWithRoot" 0 0))
    (bind _asbp_enemy_base (Utilities|Casting|CastToBP_Enemy_Base _returnvalue_2))
    (return _asbp_enemy_base)))

(fn GetClasstoSpawn
  (params (Type :type Integer))
  (return (Utilities|Select :Index (Math|Integer|Clamp(Integer) Type 0 (- (Variables|Default|GetMaxNumEnemies) 1)) :Option%200 "/Game/Blueprints/Characters/Enemies/BP_Enemy_Base.BP_Enemy_Base_C" :Option%201 "/Game/Blueprints/Characters/Enemies/BP_Enemy_H.BP_Enemy_H_C" :Option%202 "/Game/Blueprints/Characters/Enemies/BP_Enemy_S.BP_Enemy_S_C")))