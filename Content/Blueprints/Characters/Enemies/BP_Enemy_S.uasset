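; BP_Enemy_S is a space shooter enemy that moves toward the player via AI MoveTo from BeginPlay.
; An overlap passing a tag check fires the OnEnemyDestroy dispatcher and notifies BP_GameMode_SpaceShooter.
; The bound handler spawns an explosion with sound, then destroys the actor after a brief delay.
; The tag check reads the element of a TagList loop that is never executed.
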(event Custom|Follow%20Player
  ;[1 1 1] Set Event to follow Player
  (AI|AIMoveTo self "0, 0, 0" (Game|GetPlayerCharacter 0) 5.0 false))

(event Custom|Destroyed_Event
  ;[1 1 1] Set On Enemy Destroy Dispatcher
  (Effects|SpawnEmitteratLocation "/Game/StarterContent/Particles/P_Explosion.P_Explosion" (Transformation|GetActorLocation))
  (Audio|PlaySound2D "/Game/StarterContent/Audio/Explosion02.Explosion02" 0.3 1.0 0.0 0 0)
  (Utilities|FlowControl|Delay 0.1)
  (Actor|DestroyActor))

(event EventBeginPlay
  ;[1 1 1] Set On Enemy Destroy Dispatcher
  (CallFunction|FollowPlayer)
  (EventDispatchers|BindEventtoOnEnemyDestroy (delegate Custom|Destroyed_Event)))

(event Collision|EventActorBeginOverlap
  (params (OtherActor :type Actor%20Object%20Reference))
  ;[1 1 1] On collision
  (if (Utilities|Array|ContainsItem (Variables|/Script/Engine.Actor|GetTags OtherActor) (stale _array_element))
    (Default|CallOnEnemyDestroy)
    (bind _asbp_game_mode_space_shooter (Utilities|Casting|CastToBP_GameMode_SpaceShooter (Game|GetGameMode)))
    (Default|EnemyDestroyed _asbp_game_mode_space_shooter)))

(fn ConstructionScript)